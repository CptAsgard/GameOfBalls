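; AccelerationPad is a level element that boosts a BallPawn rolling into its DetectionVolume, then needs time to recharge.
; The boost projects the ball's velocity onto the pad's local XY plane, so it follows the travel direction rather than a fixed one, and adds SpeedGain along it to the PhysicsSphere.
; Charging on Tick and overlap handling both run only on the authority, with each boost resetting the charge timer.
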(event `self.ReceiveBeginPlay`)

(event `self.ReceiveTick`
  (params (DeltaSeconds :type "Float (single-precision)"))
  (bind _chargingtimer (`self.ChargingTimer`))
  (`/Engine/EditorBlueprintResources/ActorMacros.Switch Has Authority`
    (:`Authority`
      (if (not (`self.Charged`))
        (set `self.ChargingTimer` (+ DeltaSeconds _chargingtimer))
        (set `self.Charged` (> _chargingtimer (`self.RechargeTime`)))))))

(event `self.DetectionVolume.OnComponentBeginOverlap`
  (params (OtherActor :type "Actor Object Reference") (OtherComp :type "PrimitiveComponent Object Reference") (OtherBodyIndex :type Integer))
  (bind _returnvalue (`self.K2_GetActorRotation`))
  (`/Engine/EditorBlueprintResources/ActorMacros.Switch Has Authority`
    (:`Authority`
      (if (`self.Charged`)
        (`/Engine/EditorBlueprintResources/StandardMacros.IsValid` OtherActor
          (:`Is Valid`
            (bind _asballpawn_c (cast `/Game/Blueprints/Pawns/BallPawn` OtherActor))
            (bind _physicssphere (`/Game/Blueprints/Pawns/BallPawn.PhysicsSphere` _asballpawn_c))
            (`/Engine/EditorBlueprintResources/StandardMacros.IsValid` _physicssphere
              (:`Is Valid`
                (set `self.Charged` false)
                (set `self.ChargingTimer` 0.0)
                (`PrimitiveComponent.SetPhysicsLinearVelocity` _physicssphere (* (`KismetMathLibrary.Normal` (`KismetMathLibrary.GreaterGreater_VectorRotator` (`KismetMathLibrary.MakeVector` (.x (`KismetMathLibrary.LessLess_VectorRotator` (`SceneComponent.GetComponentVelocity` _physicssphere) _returnvalue)) (.y (`KismetMathLibrary.LessLess_VectorRotator` (`SceneComponent.GetComponentVelocity` _physicssphere) _returnvalue))) _returnvalue)) (`self.SpeedGain`)) true "None")))))))))

(fn `UserConstructionScript`)