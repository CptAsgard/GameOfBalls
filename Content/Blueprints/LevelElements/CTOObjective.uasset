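; Team-owned objective for a capture mode (CTO) that an opposing team's ball pawn grabs by touching its collision volume.
; On authority, an overlap records the holder, marks the objective taken and hides the mesh through a cosmetic event.
; A per-tick authority check restores the objective and mesh when the holder is invalid or no longer carries it, then rescans overlapping pawns for an immediate re-grab.
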(event `CheckObjectiveLife`
  (bind _objectiveholder (`self.ObjectiveHolder`))
  ;[0 0.7201 1] If Objective-holding pawn doesn't exist anymore or doesn't carry the objective anymore, reset availability.
  (if (not (`self.ObjectiveAvailable`))
    (`/Engine/EditorBlueprintResources/StandardMacros.IsValid` _objectiveholder
      (:`Is Valid`
        (bind _asctoplayerstate_c (cast `/Game/Blueprints/Gamemodes/CTOPlayerState` (`Pawn.PlayerState` _objectiveholder)))
        (if (not (`/Game/Blueprints/Gamemodes/CTOPlayerState.HasObjective` _asctoplayerstate_c))
          (set `self.ObjectiveAvailable` true :!label _label)
          (`self.ReturnVisualEffect`)
          (for _array_element (`PrimitiveComponent.GetOverlappingActors` (`self.CollisionVolume`) null)
            (`/Engine/EditorBlueprintResources/StandardMacros.IsValid` _array_element
              (:`Is Valid`
                (bind _asballpawn_c (cast `/Game/Blueprints/Pawns/BallPawn` _array_element))
                (set `self.ObjectiveHolder` _asballpawn_c)
                (bind _asctoplayerstate_c_2 (cast `/Game/Blueprints/Gamemodes/CTOPlayerState` (`Pawn.PlayerState` _asballpawn_c)))
                (if (!= (`/Game/Blueprints/Gamemodes/CTOPlayerState.Team` _asctoplayerstate_c_2) (`self.Team`))
                  (set `self.ObjectiveAvailable` false)
                  (set `/Game/Blueprints/Gamemodes/CTOPlayerState.HasObjective` true _asctoplayerstate_c_2)
                  (`self.CaptureVisualEffects`)))))))
      (:`Is Not Valid`
        (goto _label)))))

(event `self.ReceiveTick`
  (params (DeltaSeconds :type "Float (single-precision)"))
  ;[1 1 1] Tick
  (`|ExecutionSequence`
    (:`then_0`
      (`/Engine/EditorBlueprintResources/ActorMacros.Switch Has Authority`
        (:`Authority`
          (`self.CheckObjectiveLife`))))
    (:`then_1`
      (`/Engine/EditorBlueprintResources/StandardMacros.Can Execute Cosmetic Events`))))

(event `self.CollisionVolume.OnComponentBeginOverlap`
  (params (OtherActor :type "Actor Object Reference") (OtherComp :type "PrimitiveComponent Object Reference") (OtherBodyIndex :type Integer))
  ;[1 0.02893 0] Handle  an overlap, and see if overlapping pawn is eligible for grabbing the objective
  (`/Engine/EditorBlueprintResources/ActorMacros.Switch Has Authority`
    (:`Authority`
      (if (`self.ObjectiveAvailable`)
        (`/Engine/EditorBlueprintResources/StandardMacros.IsValid` OtherActor
          (:`Is Valid`
            (bind _asctoballpawn_c (cast `/Game/Blueprints/Pawns/CTOBallPawn` OtherActor))
            (set `self.ObjectiveHolder` _asctoballpawn_c)
            (bind _asctoplayerstate_c (cast `/Game/Blueprints/Gamemodes/CTOPlayerState` (`Pawn.PlayerState` _asctoballpawn_c)))
            (if (!= (`/Game/Blueprints/Gamemodes/CTOPlayerState.Team` _asctoplayerstate_c) (`self.Team`))
              (set `self.ObjectiveAvailable` false)
              (`/Game/Blueprints/Pawns/CTOBallPawn.SetHasObjective` _asctoballpawn_c (`self.Team`) true)
              (`self.CaptureVisualEffects`))))))))

(event `CaptureVisualEffects`
  ;[1 1 1] Play Visual effects when the flag is captured or returned
  (`/Engine/EditorBlueprintResources/StandardMacros.Can Execute Cosmetic Events`
    (:`True`
      (`SceneComponent.SetVisibility` (`self.Static Mesh`) false false))))

(event `ReturnVisualEffect`
  ;[1 1 1] Play Visual effects when the flag is captured or returned
  (`/Engine/EditorBlueprintResources/StandardMacros.Can Execute Cosmetic Events`
    (:`True`
      (`SceneComponent.SetVisibility` (`self.Static Mesh`) true false))))

(fn `UserConstructionScript`)