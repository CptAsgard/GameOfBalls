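; Game mode for the CTO mode that handles team scoring for up to four teams.
; Its ScorePoint event takes a team number and, on authority only, adds one point to that team's score on the CTOGameState.
; BeginPlay and the construction script are empty, and no win condition is checked here.
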(event `self.ReceiveBeginPlay`)

(event `ScorePoint`
  (params (Team :type Integer))
  (bind _returnvalue (`GameplayStatics.GetGameState`))
  ;[0 1 0.6984] Handle and update Scores
  (`/Engine/EditorBlueprintResources/ActorMacros.Switch Has Authority`
    (:`Authority`
      (`/Engine/EditorBlueprintResources/StandardMacros.IsValid` _returnvalue
        (:`Is Valid`
          (bind _asctogamestate_c (cast `/Game/Blueprints/Gamemodes/CTOGameState` _returnvalue))
          (if (== Team 1)
            (set `/Game/Blueprints/Gamemodes/CTOGameState.ScoreTeam1` (+ (`/Game/Blueprints/Gamemodes/CTOGameState.ScoreTeam1` _asctogamestate_c) 1) _asctogamestate_c)
            (elif (== Team 2)
              (set `/Game/Blueprints/Gamemodes/CTOGameState.ScoreTeam2` (+ (`/Game/Blueprints/Gamemodes/CTOGameState.ScoreTeam2` _asctogamestate_c) 1) _asctogamestate_c)
              (elif (== Team 3)
                (set `/Game/Blueprints/Gamemodes/CTOGameState.ScoreTeam3` (+ (`/Game/Blueprints/Gamemodes/CTOGameState.ScoreTeam3` _asctogamestate_c) 1) _asctogamestate_c)
                (elif (== Team 4)
                  (set `/Game/Blueprints/Gamemodes/CTOGameState.ScoreTeam4` (+ (`/Game/Blueprints/Gamemodes/CTOGameState.ScoreTeam4` _asctogamestate_c) 1) _asctogamestate_c))))))))))

(fn `UserConstructionScript`)