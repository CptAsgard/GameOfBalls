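; Player controller Blueprint that relays movement and camera input to the controlled BallPawn.
; Each input event checks that the controlled pawn is valid and casts it to BallPawn before forwarding the command.
; Movement axes pass their values to the pawn's forward/backward and right/left functions, while the YawLeft and YawRight presses call CameraYawSideways with a direction flag.
; The controller only routes input, leaving movement and camera logic to the pawn.
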(event `InputAxis|MoveForwardBackward`
  (params (AxisValue :type "Float (single-precision)"))
  (bind _returnvalue (`self.GetControlledPawn`))
  (`/Engine/EditorBlueprintResources/StandardMacros.IsValid` _returnvalue
    (:`Is Valid`
      (bind _asballpawn_c (cast `/Game/Blueprints/Pawns/BallPawn` _returnvalue))
      (`/Game/Blueprints/Pawns/BallPawn.MoveForwardBackward` _asballpawn_c AxisValue))))

(event `InputAxis|MoveRightLeft`
  (params (AxisValue :type "Float (single-precision)"))
  (bind _returnvalue (`self.GetControlledPawn`))
  (`/Engine/EditorBlueprintResources/StandardMacros.IsValid` _returnvalue
    (:`Is Valid`
      (bind _asballpawn_c (cast `/Game/Blueprints/Pawns/BallPawn` _returnvalue))
      (`/Game/Blueprints/Pawns/BallPawn.MoveRightLeft` _asballpawn_c AxisValue))))

(event `InputAction|YawLeft`
  (bind _returnvalue (`self.GetControlledPawn`))
  (:`Pressed`
    (`/Engine/EditorBlueprintResources/StandardMacros.IsValid` _returnvalue
      (:`Is Valid`
        (bind _asballpawn_c (cast `/Game/Blueprints/Pawns/BallPawn` _returnvalue))
        (`/Game/Blueprints/Pawns/BallPawn.CameraYawSideways` _asballpawn_c true)))))

(event `InputAction|YawRight`
  (bind _returnvalue (`self.GetControlledPawn`))
  (:`Pressed`
    (`/Engine/EditorBlueprintResources/StandardMacros.IsValid` _returnvalue
      (:`Is Valid`
        (bind _asballpawn_c (cast `/Game/Blueprints/Pawns/BallPawn` _returnvalue))
        (`/Game/Blueprints/Pawns/BallPawn.CameraYawSideways` _asballpawn_c false)))))

(fn `UserConstructionScript`)