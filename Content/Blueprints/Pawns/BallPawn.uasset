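; Physics-driven rolling ball pawn that moves under variable gravity, with a camera that follows the current "down".
; Externally supplied gravity and X vectors are averaged each authority tick, replacing world gravity and orienting input force.
; Cosmetic tick smoothly aligns the camera anchor to that frame and tilts the spring arm with local velocity.
; Manual camera yaw snaps in steps, while an automatic yaw offset compensates when entering or leaving gravity fields.
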(event `self.ReceiveBeginPlay`
  ;[1 1 1] Begin Play
  (`SceneComponent.SetAbsolute` (`self.SpringArm`) false false false)
  (`SceneComponent.SetAbsolute` (`self.Camera Anchor`) false true false))

(event `self.ReceiveTick`
  (params (DeltaSeconds :type "Float (single-precision)"))
  ;[1 1 1] Tick
  (`|ExecutionSequence`
    (:`then_0`
      (`/Engine/EditorBlueprintResources/ActorMacros.Switch Has Authority`
        (:`Authority`
          (`self.FetchVectors`)
          (`self.ApplyAcceleration`))))
    (:`then_1`
      (`/Engine/EditorBlueprintResources/StandardMacros.Can Execute Cosmetic Events`
        (:`True`
          (`self.UpdateCamera` DeltaSeconds))))))

(event `AddVectors`
  (params (GravityVector :type "Object.Vector Structure") (XVector :type "Object.Vector Structure"))
  ;[0.7299 0.5474 0] Add Gravity and X-Vector from external
  (`KismetArrayLibrary.Array_Add` (`self.GravityvectorArray`) GravityVector)
  (`KismetArrayLibrary.Array_Add` (`self.XVectorArray`) XVector)
  (set `self.InGravityWall` true))

(event `FetchVectors`
  (bind _physicssphere (`self.PhysicsSphere`))
  (bind _physicssphere_2 (`self.PhysicsSphere`))
  (bind _gravityvectorarray (`self.GravityvectorArray`))
  (bind _xvectorarray (`self.XVectorArray`))
  (bind _physicssphere_3 (`self.PhysicsSphere`))
  ;[0.7299 0.5328 0] Fetch Gravityvector and X-Vector for Gravity and Camera Management
  (if (`self.InGravityWall`)
    ;;[1 1 1] If pawn is in gravity field
    (set `self.InGravityWall` false)
    (`|ExecutionSequence`
      (:`then_0`
        (`/Engine/EditorBlueprintResources/StandardMacros.IsValid` _physicssphere_3
          (:`Is Valid`
            (`PrimitiveComponent.SetEnableGravity` _physicssphere_3 false)
            (set `self.Gravityvector` (0.0 0.0 0.0))
            (set `self.XVector` (0.0 0.0 0.0))
            (for _array_element _gravityvectorarray
              (set `self.Gravityvector` (+ _array_element (`self.Gravityvector`))))
            (set `self.Gravityvector` (/ (`self.Gravityvector`) (`KismetMathLibrary.Conv_IntToDouble` (`KismetArrayLibrary.Array_Length` _gravityvectorarray))))
            (`KismetArrayLibrary.Array_Clear` _gravityvectorarray)
            (for _array_element_2 _xvectorarray
              (set `self.XVector` (+ _array_element_2 (`self.XVector`))))
            (set `self.XVector` (/ (`self.XVector`) (`KismetMathLibrary.Conv_IntToDouble` (`KismetArrayLibrary.Array_Length` _xvectorarray))))
            (`KismetArrayLibrary.Array_Clear` _xvectorarray)
            (`|ExecutionSequence`
              (:`then_0`
                (`/Engine/EditorBlueprintResources/StandardMacros.DoOnce` false :!label _label
                  (:`Completed`
                    (set `self.CameraYawRotationAuto` (- (- (`self.CameraYawRotationAuto`) (`self.CameraYawRotation`)) (- (`KismetMathLibrary.DegAtan2` (.y (`self.XVector`)) (.x (`self.XVector`))) (`self.CameraYawRotation`)))))))
              (:`then_1`
                (set `self.XVector` (`KismetMathLibrary.RotateAngleAxis` (`self.XVector`) (+ (`self.CameraYawRotation`) (`self.CameraYawRotationAuto`)) (* (`self.Gravityvector`) -1.0)))
                (`PrimitiveComponent.AddForce` _physicssphere (* (* (`self.Gravityvector`) 980.0) (`PrimitiveComponent.GetMass` _physicssphere)) "None"))))))
      (:`then_1`
        (goto _label_2 :!via `Reset`))
      (:`then_2`
        (goto _label_3 :!via `Reset`)))
    (else
      ;;[1 1 1] If Pawn isn't in Gravity Field
      (`|ExecutionSequence`
        (:`then_0`
          (`/Engine/EditorBlueprintResources/StandardMacros.DoOnce` false :!label _label_2
            (:`Completed`
              (set `self.CameraYawRotationAuto` (- (`KismetMathLibrary.DegAtan2` (.y (`self.XVector`)) (.x (`self.XVector`))) (`self.CameraYawRotation`))))))
        (:`then_1`
          (`/Engine/EditorBlueprintResources/StandardMacros.IsValid` _physicssphere_2
            (:`Is Valid`
              (`PrimitiveComponent.SetEnableGravity` _physicssphere_2 true)
              (set `self.Gravityvector` (0.0 0.0 -1.0))
              (set `self.XVector` (`KismetMathLibrary.RotateAngleAxis` (1.0 0.0 0.0) (+ (`self.CameraYawRotationAuto`) (`self.CameraYawRotation`)) (0.0 0.0 1.0)))
              (goto _label :!via `Reset`))))
        (:`then_2`
          (`/Engine/EditorBlueprintResources/StandardMacros.DoOnce` false :!label _label_3))))))

(event `UpdateCamera`
  (params (`Delta Time` :type "Float (double-precision)"))
  (bind _xvector (`self.XVector`))
  (bind _gravityvector (`self.Gravityvector`))
  (bind _springarm (`self.SpringArm`))
  (bind _cameratiltvelocity (`self.CameraTiltVelocity`))
  (bind _camera_anchor (`self.Camera Anchor`))
  (bind _returnvalue (`KismetMathLibrary.FClamp` (/ (.x (`KismetMathLibrary.LessLess_VectorRotator` (`SceneComponent.GetComponentVelocity` (`self.PhysicsSphere`)) (`KismetMathLibrary.MakeRotFromZX` (* (`self.Gravityvector`) -1.0) (`self.XVector`)))) _cameratiltvelocity) -1.0))
  (bind _returnvalue_2 (`KismetMathLibrary.FClamp` (/ (.y (`KismetMathLibrary.LessLess_VectorRotator` (`SceneComponent.GetComponentVelocity` (`self.PhysicsSphere`)) (`KismetMathLibrary.MakeRotFromZX` (* (`self.Gravityvector`) -1.0) (`self.XVector`)))) _cameratiltvelocity) -1.0))
  ;[0.1762 1 0.1714] Camera Rotation
  (`SceneComponent.SetRelativeRotation` _springarm (`KismetMathLibrary.RInterpTo` (`SceneComponent.RelativeRotation` _springarm) (`KismetMathLibrary.MakeRot` (+ (`KismetMathLibrary.Lerp` 0.0 30.0 (* (`KismetMathLibrary.MultiplyMultiply_FloatFloat` (`KismetMathLibrary.Abs` _returnvalue) 1.5) (`KismetMathLibrary.SignOfFloat` _returnvalue))) -45.0 (`KismetMathLibrary.Lerp` 0.0 10.0 (`KismetMathLibrary.FClamp` (/ (.z (`KismetMathLibrary.LessLess_VectorRotator` (`SceneComponent.GetComponentVelocity` (`self.PhysicsSphere`)) (`KismetMathLibrary.MakeRotFromZX` (* (`self.Gravityvector`) -1.0) (`self.XVector`)))) _cameratiltvelocity) -1.0))) (`KismetMathLibrary.Lerp` 0.0 30.0 (* (`KismetMathLibrary.MultiplyMultiply_FloatFloat` (`KismetMathLibrary.Abs` _returnvalue_2) 1.5) (`KismetMathLibrary.SignOfFloat` _returnvalue_2)))) `Delta Time` 3.0) false)
  (`SceneComponent.SetRelativeRotation` _camera_anchor (`KismetMathLibrary.RInterpTo` (`SceneComponent.RelativeRotation` _camera_anchor) (`KismetMathLibrary.MakeRotationFromAxes` _xvector (`KismetMathLibrary.Cross_VectorVector` _xvector _gravityvector) (* _gravityvector -1.0)) `Delta Time` 5.0) false))

(event `CameraYawSideways`
  (params (Left :type Boolean))
  (bind _camerayawsnapangle (`self.CameraYawSnapAngle`))
  (bind _camerayawsnapangle_2 (`self.CameraYawSnapAngle`))
  (bind _returnvalue (+ (`self.CameraYawRotationAuto`) (`self.CameraYawRotation`)))
  (bind _returnvalue_2 (/ _returnvalue (`self.CameraYawSnapAngle`)))
  (bind _returnvalue_3 (mod _returnvalue (`self.CameraYawSnapAngle`)))
  (bind _returnvalue_4 (* (`KismetMathLibrary.FFloor` _returnvalue_2) _camerayawsnapangle_2))
  (bind _returnvalue_5 (* (`KismetMathLibrary.FCeil` _returnvalue_2) _camerayawsnapangle_2))
  ;[0.1762 1 0.1714] Camera Rotation
  ;;[1 1 1] Rotate Camera Yaw on User Input
  (if Left
    (`/Engine/EditorBlueprintResources/StandardMacros.CompareFloat` _returnvalue_3
      (:`>`
        (set `self.CameraYawRotation` _returnvalue_5 :!label _label_4))
      (:`==`
        (set `self.CameraYawRotation` (+ _returnvalue_5 _camerayawsnapangle)))
      (:`<`
        (goto _label_4)))
    (else
      (`/Engine/EditorBlueprintResources/StandardMacros.CompareFloat` _returnvalue_3
        (:`>`
          (set `self.CameraYawRotation` _returnvalue_4 :!label _label_5))
        (:`==`
          (set `self.CameraYawRotation` (- _returnvalue_4 _camerayawsnapangle)))
        (:`<`
          (goto _label_5)))))
  (set `self.CameraYawRotationAuto` 0.0))

(event `ApplyAcceleration`
  (bind _xvector (`self.XVector`))
  (bind _gravityvector (`self.Gravityvector`))
  (bind _returnvalue (`KismetMathLibrary.MakeVector` (`self.InputForwardBackward`) (`self.InputRightLeft`)))
  ;[1 1 1] Movement
  (if (>= (`KismetMathLibrary.VSize` _returnvalue) 1.0)
    (set `self.AccelerationDirection` (`KismetMathLibrary.Normal` _returnvalue))
    (else
      (set `self.AccelerationDirection` _returnvalue)))
  (`PrimitiveComponent.AddForce` (`self.PhysicsSphere`) (* (* (`KismetMathLibrary.GreaterGreater_VectorRotator` (`self.AccelerationDirection`) (`KismetMathLibrary.MakeRotationFromAxes` _xvector (`KismetMathLibrary.Cross_VectorVector` _xvector _gravityvector) (* _gravityvector -1.0))) (* (`self.BallAcceleration`) (`self.BallAccelerationMultiplier`))) (`PrimitiveComponent.GetMass` (`self.PhysicsSphere`))) "None"))

(event `MoveForwardBackward`
  (params (Amount :type "Float (double-precision)"))
  ;[1 1 1] Movement
  (`/Engine/EditorBlueprintResources/ActorMacros.Switch Has Authority`
    (:`Authority`
      (set `self.InputForwardBackward` Amount))))

(event `MoveRightLeft`
  (params (Amount :type "Float (double-precision)"))
  ;[1 1 1] Movement
  (`/Engine/EditorBlueprintResources/ActorMacros.Switch Has Authority`
    (:`Authority`
      (set `self.InputRightLeft` Amount))))

(fn `UserConstructionScript`)