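; Player ball pawn for the CTO mode, handling movement, camera updates and objective possession.
; Each tick, the server runs FetchVectors and ApplyAcceleration, while UpdateCamera runs only where cosmetic events can execute.
; At BeginPlay the CameraAnchor gets absolute rotation, decoupling it from parent rotation, while the SpringArm stays fully relative.
; SetHasObjective writes possession and team to CTOPlayerState on the server; its final possession branch is empty.
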(event `self.ReceiveBeginPlay`
  ;[0.966 1 0] Begin Play
  (`SceneComponent.SetAbsolute` (`self.SpringArm`) false false false)
  (`SceneComponent.SetAbsolute` (`self.Camera Anchor`) false true false))

(event `self.ReceiveTick`
  (params (DeltaSeconds :type "Float (single-precision)"))
  ;[0 0.3629 1] Tick
  (`|ExecutionSequence`
    (:`then_0`
      (`/Engine/EditorBlueprintResources/ActorMacros.Switch Has Authority`
        (:`Authority`
          (`self.FetchVectors`)
          (`self.ApplyAcceleration`))))
    (:`then_1`
      (`/Engine/EditorBlueprintResources/StandardMacros.Can Execute Cosmetic Events`
        (:`True`
          (`self.UpdateCamera` DeltaSeconds))))))

(event `SetHasObjective`
  (params (Team :type Integer) (HasObjective :type Boolean))
  ;[0 1 0.171] Handling capture and loss of the objective
  (`/Engine/EditorBlueprintResources/ActorMacros.Switch Has Authority`
    (:`Authority`
      (bind _asctoplayerstate_c (cast `/Game/Blueprints/Gamemodes/CTOPlayerState` (`self.PlayerState`)))
      (set `/Game/Blueprints/Gamemodes/CTOPlayerState.HasObjective` HasObjective _asctoplayerstate_c)
      (set `/Game/Blueprints/Gamemodes/CTOPlayerState.ObjectiveTeam` Team _asctoplayerstate_c)
      (if HasObjective
        _))))

(fn `UserConstructionScript`
  (`parent.UserConstructionScript`))